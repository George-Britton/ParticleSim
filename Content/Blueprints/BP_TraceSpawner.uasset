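; BP_TraceSpawner fills a box volume with randomly moving BP_Trace actors.
; Init stores the count, speed range, scale, box size and emissive value, resizes the Box and calls Go.
; Go spawns each trace at a random point in the box, giving valid ones a random speed and normalized direction, then initializing their emissive.
; The construction script keeps MaxSpeed at or above MinSpeed and syncs the box extent.
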(event `Init`
  (params (NumberOfTraces :type Integer) (MinSpeed :type "Float (double-precision)") (MaxSpeed :type "Float (double-precision)") (TraceScale :type "Float (double-precision)") (Size :type "Vector Structure") (Emissive :type "Float (double-precision)"))
  (set `self.NumOfTraces` NumberOfTraces)
  (set `self.MinSpeed` MinSpeed)
  (set `self.MaxSpeed` MaxSpeed)
  (set `self.TraceScale` TraceScale)
  (bind _output_get (set `self.BoxExtent` Size))
  (set `self.Emissive` Emissive)
  (`BoxComponent.SetBoxExtent` (`self.Box`) _output_get true)
  (`self.Go`))

(event `Go`
  (bind _box (`self.Box`))
  (for _ (range (`self.NumOfTraces`))
    (bind _returnvalue (`|SpawnActorFromClass` "/Game/Blueprints/BP_Trace.BP_Trace_C" (`KismetMathLibrary.MakeTransform` (`KismetMathLibrary.RandomPointInBoundingBox` (`SceneComponent.K2_GetComponentLocation` _box) (`BoxComponent.BoxExtent` _box)) (struct) (`KismetMathLibrary.Conv_DoubleToVector` (`self.TraceScale`))) "AdjustIfPossibleButDontSpawnIfColliding" "OverrideRootScale" null null))
    (`/Engine/EditorBlueprintResources/StandardMacros.IsValid` _returnvalue
      (:`Is Valid`
        (set `/Game/Blueprints/BP_Trace.Speed` (`KismetMathLibrary.RandomFloatInRange` (`self.MinSpeed`) (`self.MaxSpeed`)) _returnvalue)
        (set `/Game/Blueprints/BP_Trace.Velocity` (`KismetMathLibrary.Normal` (`KismetMathLibrary.MakeVector` (`KismetMathLibrary.RandomFloatInRange` -1.0 1.0) (`KismetMathLibrary.RandomFloatInRange` -1.0 1.0) (`KismetMathLibrary.RandomFloatInRange` -1.0 1.0))) _returnvalue)
        (`/Game/Blueprints/BP_Trace.Init` _returnvalue (`self.Emissive`))))))

(fn `UserConstructionScript`
  (set `self.MaxSpeed` (`KismetMathLibrary.FClamp` (`self.MaxSpeed`) (`self.MinSpeed`) 9999999.0))
  (`BoxComponent.SetBoxExtent` (`self.Box`) (`self.BoxExtent`) true))