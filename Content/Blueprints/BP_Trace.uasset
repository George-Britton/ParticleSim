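; BP_Trace is a moving particle actor that bounces off surfaces and records each contact point.
; Each tick it sweeps along its normalized Velocity at Speed and turns to face its heading.
; Hits on WorldStatic or GameTraceChannel1 objects halt it, then reflect the saved velocity using the actor-relative impact point as normal.
; A dynamic material gets a random colour; ChangeColour rerolls it and toggles emissive, but its looping timer is unconnected.
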(event `Init`
  (params (Emissive :type "Float (double-precision)"))
  (set `self.Emissive` Emissive)
  (`self.Start`))

(event `Start`
  (bind _returnvalue (`PrimitiveComponent.CreateDynamicMaterialInstance` (`self.Particle`) 0 "/Game/Materials/M_Master.M_Master" "None"))
  (bind _output_get (set `self.DMI` _returnvalue))
  (`MaterialInstanceDynamic.SetVectorParameterValue` _output_get "Colour" (`self.RandomColour` 1.0))
  (`KismetArrayLibrary.Array_Add` (`self.ContactPoints`) (`self.K2_GetActorLocation`))
  (`MaterialInstanceDynamic.SetScalarParameterValue` _output_get "Emissive" (`self.Emissive`)))

(event `ChangeColour`
  (bind _dmi (`self.DMI`))
  ;[1 1 1] Connect to party
  (`MaterialInstanceDynamic.SetVectorParameterValue` _dmi "Colour" (`self.RandomColour` 1.0))
  (bind _returnvalue (`MaterialInstanceDynamic.K2_GetScalarParameterValue` _dmi "Emissive"))
  (`MaterialInstanceDynamic.SetScalarParameterValue` _dmi "Emissive" (* (`KismetMathLibrary.Conv_BoolToDouble` (== _returnvalue 0.0)) 10.0)))

(event `self.ReceiveTick`
  (params (DeltaSeconds :type "Float (single-precision)"))
  (`self.Move`)
  (if (not (`self.IsStationary`))
    (`self.Face Forward`)))

(event `self.Particle.OnComponentHit`
  (params (HitComponent :type "PrimitiveComponent Object Reference") (OtherActor :type "Actor Object Reference") (OtherComp :type "PrimitiveComponent Object Reference") (NormalImpulse :type "Vector Structure") (Hit :type "HitResult Structure (by ref)"))
  (bind _returnvalue (`PrimitiveComponent.GetCollisionObjectType` OtherComp))
  (if (or (`|EnumEquality` _returnvalue "ECC_WorldStatic") (`|EnumEquality` _returnvalue "ECC_GameTraceChannel1"))
    (`self.Collide` (`PrimitiveComponent.GetClosestPointOnCollision` OtherComp (`self.K2_GetActorLocation`) "None"))))

(fn `Collide`
  (params (ImpactPoint :type "Vector Structure"))
  (locals (NewX :type "Float (double-precision)") (NewY :type "Float (double-precision)") (NewZ :type "Float (double-precision)") (NewVel :type "Vector Structure") (IPD :type "Float (double-precision)") (ForwardDistance :type "Vector Structure") (RotationToAdd :type "Rotator Structure" :default (struct)) (temp :type "Rotator Structure" :default (struct)) (Mirror :type "/Game/Blueprints/BP_Mirror Object Reference"))
  (set `self.ImpactPoint` ImpactPoint)
  (`|ExecutionSequence`
    (:`then_0`
      (`self.AddPointToArray` (`local.ImpactPoint`))
      (bind _ipr (`self.GetRelativeImpactPoint` (`local.ImpactPoint`)))
      (set `self.IPR` _ipr)
      (bind _distance (`self.GetDistanceToImpactPoint`))
      (set `local.IPD` _distance)
      (bind _forwardprojection (`self.ProjectForwardByDistance`))
      (set `local.ForwardDistance` _forwardprojection)
      (`self.Halt`))
    (:`then_1`
      (bind _output_get (set `self.MirrorredVelocity` (`self.SavedVelocity`)))
      (`self.Go` false (`KismetMathLibrary.GetReflectionVector` _output_get (`self.IPR`))))))

(fn `Go`
  (params (ResumePrevious :type Boolean) (NewVelocity :type "Vector Structure"))
  (if ResumePrevious
    (set `self.Velocity` (`self.SavedVelocity`))
    (else
      (set `self.Velocity` NewVelocity)))
  (return))

(fn `Halt`
  (set `self.SavedVelocity` (`self.Velocity`))
  (set `self.Velocity` (0.0 0.0 0.0))
  (return))

(fn `UserConstructionScript`)