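; Maze actor that builds a grid level for a trace-based pathfinding run, optionally using customised layout and trace settings from GI_Maze.
; It spawns wall meshes for false cells, places start, end, floor, ceiling and a side cap, then frames an orthographic camera.
; BP_TraceSpawner starts at the start and BP_Goal at the end.
; When the goal broadcasts a path, all traces are destroyed, BP_Path draws it and a restart widget appears.
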(event `self.ReceiveBeginPlay`
  (bind _asgi_maze (cast `/Game/Config/GI_Maze` (`GameplayStatics.GetGameInstance`)))
  (if (`/Game/Config/GI_Maze.Customised` _asgi_maze)
    (set `self.GridMap` (`/Game/Config/GI_Maze.Grid` _asgi_maze))
    (set `self.StartVec` (`/Game/Config/GI_Maze.Start` _asgi_maze))
    (set `self.GoalVec` (`/Game/Config/GI_Maze.End` _asgi_maze))
    (`self.Init` (`/Game/Config/GI_Maze.Num` _asgi_maze) (`/Game/Config/GI_Maze.Min` _asgi_maze) (`/Game/Config/GI_Maze.Max` _asgi_maze) (`/Game/Config/GI_Maze.Scale` _asgi_maze) (`/Game/Config/GI_Maze.Emissive` _asgi_maze))
    (else
      (`self.Begin`))))

(event `Init`
  (params (Number :type Integer) (MinSpeed :type "Float (double-precision)") (MaxSpeed :type "Float (double-precision)") (Scale :type "Float (double-precision)") (Emissive :type "Float (double-precision)"))
  (set `self.NumberOfTraces` Number)
  (set `self.MinSpeed` MinSpeed)
  (set `self.MaxSpeed` MaxSpeed)
  (set `self.TraceScale` (* Scale 0.03))
  (set `self.Emissive` Emissive)
  (`self.Begin`))

(event `Begin`
  (bind _camera (`self.Camera`))
  (bind _gridmap (`self.GridMap`))
  (bind _returnvalue (`KismetArrayLibrary.Array_Length` _gridmap))
  (bind (_returnvalue_origin _returnvalue_boxextent) (`KismetMathLibrary.BreakBoxSphereBounds` (`StaticMesh.GetBounds` (`self.GridMesh`))))
  (bind _output_row (break `/Game/Config/Row` (`|GetArrayItem` _gridmap)))
  (bind _cameracomponent (`CameraActor.CameraComponent` _camera))
  (bind _returnvalue_2 (`KismetArrayLibrary.Array_Length` _output_row))
  (`self.Make`)
  (bind _returnvalue_3 (`GameplayStatics.GetActorOfClass` "/Script/Engine.CameraActor"))
  (set `self.Camera` _returnvalue_3)
  (bind _returnvalue_4 (`|SpawnActorFromClass` "/Game/Blueprints/Actors/BP_Goal.BP_Goal_C" (`KismetMathLibrary.MakeTransform` (`SceneComponent.K2_GetComponentLocation` (`self.End`))) "Undefined" "OverrideRootScale" null null))
  (`/Game/Blueprints/Actors/BP_Goal.Init` _returnvalue_4 _returnvalue_boxextent)
  (bind _returnvalue_5 (`|SpawnActorFromClass` "/Game/Blueprints/Actors/BP_TraceSpawner.BP_TraceSpawner_C" (`KismetMathLibrary.MakeTransform` (`SceneComponent.K2_GetComponentLocation` (`self.Start`))) "Undefined" "OverrideRootScale" null null))
  (`/Game/Blueprints/Actors/BP_TraceSpawner.Init` _returnvalue_5 (`self.NumberOfTraces`) (`self.MinSpeed`) (`self.MaxSpeed`) (`self.TraceScale`) (* _returnvalue_boxextent 0.9) (`self.Emissive`))
  (`CameraComponent.SetOrthoWidth` _cameracomponent (`KismetMathLibrary.Conv_IntToDouble` (* _returnvalue _returnvalue_2 25)))
  (`SceneComponent.K2_AddWorldOffset` _cameracomponent (`KismetMathLibrary.MakeVector` (`KismetMathLibrary.Conv_IntToDouble` (* _returnvalue_2 50)) (`KismetMathLibrary.Conv_IntToDouble` (* _returnvalue 50)) (`KismetMathLibrary.Conv_IntToDouble` (* _returnvalue 200))) false true)
  (`PlayerController.SetViewTargetWithBlend` (`GameplayStatics.GetPlayerController` 0) _camera 0.0 "VTBlend_Linear" 0.0 false)
  (`self.Bind`))

(event `Bind`
  (bind _returnvalue (`GameplayStatics.GetActorOfClass` "/Game/Blueprints/Actors/BP_Goal.BP_Goal_C"))
  (add `/Game/Blueprints/Actors/BP_Goal.MakeThisPath` _returnvalue (delegate `MakeThisPath_Event_0`)))

(event `MakeThisPath_Event_0`
  (params (Path :type "Array of Vector Structure (by ref)"))
  (bind _outactors (`GameplayStatics.GetAllActorsOfClass` "/Game/Blueprints/Actors/BP_Trace.BP_Trace_C"))
  (set `self.Path` Path)
  (for _array_element _outactors
    (`self.K2_DestroyActor` _array_element))
  (bind _returnvalue (`|SpawnActorFromClass` "/Game/Blueprints/Actors/BP_Path.BP_Path_C" (`KismetMathLibrary.MakeTransform` (`|GetArrayItem` (`self.Path`))) "Undefined" "OverrideRootScale" null null))
  (`/Game/Blueprints/Actors/BP_Path.CreatePath` _returnvalue (`self.Path`))
  (bind _returnvalue_2 (`|CreateWidget` "/Game/Blueprints/Widgets/WBP_Restart.WBP_Restart_C"))
  (`UserWidget.AddToViewport` _returnvalue_2 0))

(fn `CapSides`
  (locals (Cap :type "StaticMeshComponent Object Reference"))
  (bind _startcap (`self.StartCap`))
  (bind _startcap_2 (`self.StartCap`))
  (bind _output_row (break `/Game/Config/Row` (`|GetArrayItem` (`self.GridMap`))))
  (bind (_relativescale3d_x _relativescale3d_y) (`KismetMathLibrary.BreakVector` (`SceneComponent.RelativeScale3D` _startcap)))
  (bind _relativescale3d_x_2 (`KismetMathLibrary.BreakVector` (`SceneComponent.RelativeScale3D` _startcap_2)))
  (bind _returnvalue (`StaticMesh.GetBounds` (`StaticMeshComponent.StaticMesh` _startcap)))
  (bind _returnvalue_2 (`KismetMathLibrary.Conv_IntToDouble` (`KismetArrayLibrary.Array_Length` _output_row)))
  (`StaticMeshComponent.SetStaticMesh` (`self.StartCap`) "/Game/StarterContent/Shapes/Shape_Cube.Shape_Cube")
  (`SceneComponent.SetRelativeScale3D` (`self.StartCap`) (`KismetMathLibrary.MakeVector` 0.1 _returnvalue_2 1.0))
  (`SceneComponent.K2_AddLocalOffset` (`self.StartCap`) (`KismetMathLibrary.MakeVector` (- (* _relativescale3d_x (.x (`.BoxExtent` (`KismetMathLibrary.BreakBoxSphereBounds` _returnvalue))) -1.0) (.z (`.BoxExtent` (`KismetMathLibrary.BreakBoxSphereBounds` _returnvalue)))) (* _returnvalue_2 _relativescale3d_y 4.5)) false true)
  (`SceneComponent.K2_AddWorldOffset` (`self.StartCap`) (`KismetMathLibrary.MakeVector` (* (.x (`.BoxExtent` (`KismetMathLibrary.BreakBoxSphereBounds` (`StaticMesh.GetBounds` (`self.GridMesh`))))) -2.0)) false false)
  (`SceneComponent.K2_AddWorldOffset` (`self.StartCap`) (`KismetMathLibrary.MakeVector` (* (.x (`.BoxExtent` (`KismetMathLibrary.BreakBoxSphereBounds` (`StaticMesh.GetBounds` (`StaticMeshComponent.StaticMesh` _startcap_2))))) _relativescale3d_x_2 -2.0)) false false))

(fn `CreateFloorAndCeiling`
  (bind _gridmap (`self.GridMap`))
  (bind _ceiling (`self.Ceiling`))
  (bind _floor (`self.Floor`))
  (bind _returnvalue (`KismetArrayLibrary.Array_Length` _gridmap))
  (bind _returnvalue_2 (`StaticMesh.GetBounds` (`self.GridMesh`)))
  (bind _output_row (break `/Game/Config/Row` (`|GetArrayItem` _gridmap)))
  (bind (_relativescale3d_x _relativescale3d_y _relativescale3d_z) (`KismetMathLibrary.BreakVector` (`SceneComponent.RelativeScale3D` _floor)))
  (bind _returnvalue_3 (`StaticMesh.GetBounds` (`StaticMeshComponent.StaticMesh` _floor)))
  (bind _returnvalue_4 (`KismetMathLibrary.Conv_IntToDouble` _returnvalue))
  (bind _returnvalue_5 (`KismetMathLibrary.Conv_IntToDouble` (`KismetArrayLibrary.Array_Length` _output_row)))
  (bind _returnvalue_6 (* (.z (`.BoxExtent` (`KismetMathLibrary.BreakBoxSphereBounds` _returnvalue_3))) _relativescale3d_z))
  (bind _returnvalue_7 (* _returnvalue_6 -1.0))
  (`SceneComponent.SetRelativeScale3D` _ceiling (`KismetMathLibrary.MakeVector` _returnvalue_4 _returnvalue_5 0.1))
  (`SceneComponent.SetRelativeScale3D` (`self.Floor`) (`KismetMathLibrary.MakeVector` _returnvalue_4 _returnvalue_5 0.1))
  (`SceneComponent.K2_AddLocalOffset` (`self.Floor`) (`KismetMathLibrary.MakeVector` (- (* _returnvalue_4 (.x (`.BoxExtent` (`KismetMathLibrary.BreakBoxSphereBounds` _returnvalue_2)))) (.y (`.BoxExtent` (`KismetMathLibrary.BreakBoxSphereBounds` _returnvalue_2)))) (- (* _returnvalue_5 (.y (`.BoxExtent` (`KismetMathLibrary.BreakBoxSphereBounds` _returnvalue_2)))) (.y (`.BoxExtent` (`KismetMathLibrary.BreakBoxSphereBounds` _returnvalue_2)))) _returnvalue_6) false true)
  (`SceneComponent.K2_AddLocalOffset` _ceiling (`KismetMathLibrary.MakeVector` (- (* _returnvalue_4 (.x (`.BoxExtent` (`KismetMathLibrary.BreakBoxSphereBounds` _returnvalue_2)))) (.y (`.BoxExtent` (`KismetMathLibrary.BreakBoxSphereBounds` _returnvalue_2)))) (- (* _returnvalue_5 (.y (`.BoxExtent` (`KismetMathLibrary.BreakBoxSphereBounds` _returnvalue_2)))) (.y (`.BoxExtent` (`KismetMathLibrary.BreakBoxSphereBounds` _returnvalue_2)))) _returnvalue_6) false true)
  (`SceneComponent.K2_AddLocalOffset` _ceiling (`KismetMathLibrary.MakeVector` 0.0 0.0 (+ (.z (`.BoxExtent` (`KismetMathLibrary.BreakBoxSphereBounds` _returnvalue_2))) (.z (`.BoxExtent` (`KismetMathLibrary.BreakBoxSphereBounds` _returnvalue_2))) _returnvalue_7 _returnvalue_7)) false true)
  (`SceneComponent.K2_AddLocalOffset` _ceiling (`KismetMathLibrary.MakeVector` (* (- _returnvalue 1) (.x (`.BoxExtent` (`KismetMathLibrary.BreakBoxSphereBounds` _returnvalue_3))) -2.0)) false false)
  (`SceneComponent.K2_AddLocalOffset` (`self.Floor`) (`KismetMathLibrary.MakeVector` (* (- _returnvalue 1) (.x (`.BoxExtent` (`KismetMathLibrary.BreakBoxSphereBounds` _returnvalue_3))) -2.0)) false false)
  (`SceneComponent.K2_AddWorldOffset` (`self.DefaultSceneRoot`) (`KismetMathLibrary.MakeVector` 0.0 0.0 (* (.z (`.BoxExtent` (`KismetMathLibrary.BreakBoxSphereBounds` _returnvalue_2))) 2.0)) false false)
  (`SceneComponent.K2_AddWorldOffset` (`self.Floor`) (`KismetMathLibrary.MakeVector` 0.0 0.0 (* (.z (`.BoxExtent` (`KismetMathLibrary.BreakBoxSphereBounds` _returnvalue_3))) _relativescale3d_z 2.0)) false true)
  (`SceneComponent.K2_AddWorldOffset` (`self.Ceiling`) (`KismetMathLibrary.MakeVector` 0.0 0.0 (* (.z (`.BoxExtent` (`KismetMathLibrary.BreakBoxSphereBounds` _returnvalue_3))) _relativescale3d_z -2.0)) false false))

(fn `CreateMap`
  (locals (RowNum :type Integer) (ColumnNum :type Integer))
  (for (_array_element _array_index) (`self.GridMap`)
    (set `local.ColumnNum` _array_index)
    (for (_array_element_2 _array_index_2) (`.Row_3_1333EE014BEF9CD1A6CDC786DFF18153` (break `/Game/Config/Row` _array_element))
      (set `local.RowNum` _array_index_2)
      (if (not _array_element_2)
        (bind _returnvalue (`|SpawnActorFromClass` "/Script/Engine.StaticMeshActor" (`KismetMathLibrary.MakeTransform` (`self.GetWallLocation` (`local.RowNum`) (`local.ColumnNum`))) "AlwaysSpawn" "OverrideRootScale" null null))
        (`StaticMeshComponent.SetStaticMesh` (`StaticMeshActor.StaticMeshComponent` _returnvalue) (`self.GridMesh`))
        (bind _staticmeshcomponent (`StaticMeshActor.StaticMeshComponent` _returnvalue))
        (`PrimitiveComponent.SetCollisionObjectType` _staticmeshcomponent "ECC_WorldStatic")
        (`PrimitiveComponent.SetCollisionResponseToAllChannels` _staticmeshcomponent "ECR_Block")
        (`SceneComponent.SetVisibility` _staticmeshcomponent true false))))
  (return))

(fn `Make`
  (`self.CreateMap`)
  (`self.MakeStart`)
  (`self.MakeEnd`)
  (`self.CreateFloorAndCeiling`)
  (`self.CapSides`)
  (return))

(fn `MakeEnd`
  (bind _gridmap (`self.GridMap`))
  (bind _goalvec (`self.GoalVec`))
  (bind _returnvalue (`StaticMesh.GetBounds` (`self.GridMesh`)))
  (bind _output_row (break `/Game/Config/Row` (`|GetArrayItem` _gridmap)))
  (bind _returnvalue_2 (mod _goalvec (`KismetArrayLibrary.Array_Length` _output_row)))
  (`SceneComponent.K2_SetRelativeLocation` (`self.End`) (+ (- (`SceneComponent.RelativeLocation` (`self.End`)) (`KismetMathLibrary.MakeVector` (* _returnvalue_2 (.x (`.BoxExtent` (`KismetMathLibrary.BreakBoxSphereBounds` _returnvalue))) 2.0) (* (/ (- _goalvec _returnvalue_2) (`KismetArrayLibrary.Array_Length` _gridmap)) (.y (`.BoxExtent` (`KismetMathLibrary.BreakBoxSphereBounds` _returnvalue))) -2.0))) (`KismetMathLibrary.MakeVector` 0.0 0.0 (/ (`.SphereRadius` (`KismetMathLibrary.BreakBoxSphereBounds` (`StaticMesh.GetBounds` (`self.GridMesh`)))) 2.0))) false true)
  (return))

(fn `MakeStart`
  (bind _gridmap (`self.GridMap`))
  (bind _startvec (`self.StartVec`))
  (bind _returnvalue (`StaticMesh.GetBounds` (`self.GridMesh`)))
  (bind _output_row (break `/Game/Config/Row` (`|GetArrayItem` _gridmap)))
  (bind _returnvalue_2 (mod _startvec (`KismetArrayLibrary.Array_Length` _output_row)))
  (`SceneComponent.K2_SetRelativeLocation` (`self.Start`) (+ (- (`SceneComponent.RelativeLocation` (`self.Start`)) (`KismetMathLibrary.MakeVector` (* _returnvalue_2 (.x (`.BoxExtent` (`KismetMathLibrary.BreakBoxSphereBounds` _returnvalue))) 2.0) (* (/ (- _startvec _returnvalue_2) (`KismetArrayLibrary.Array_Length` _gridmap)) (.y (`.BoxExtent` (`KismetMathLibrary.BreakBoxSphereBounds` _returnvalue))) -2.0))) (`KismetMathLibrary.MakeVector` 0.0 0.0 (/ (`.SphereRadius` (`KismetMathLibrary.BreakBoxSphereBounds` (`StaticMesh.GetBounds` (`self.GridMesh`)))) 2.0))) false true)
  (return))

(fn `UserConstructionScript`)